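; Base Blueprint for obtainable items, with a mesh set from ItemModel at construction and a name and description to report.
; ObtainItem looks up BP_TextHolder_Parent actors and uses UniversalStateSetter to reset the first one's unique state to 0, returning from inside the loop.
; It also triggers DestroyItem, which removes the actor after a short delay, and returns the item's name and description to the caller.
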(event `DestroyItem`
  (`KismetSystemLibrary.Delay` 0.1)
  (`self.K2_DestroyActor`))

(fn `ObtainItem`
  (returns (ItemName :type String) (ItemDesciption :type String))
  ;[1 1 1] Change the state of one character
  (bind _outactors (`GameplayStatics.GetAllActorsOfClass` "/Game/Blueprints/Interactables/TextHolders/BP_TextHolder_Parent.BP_TextHolder_Parent_C"))
  (for _array_element _outactors
    (bind _asbp_text_holder_parent (cast `/Game/Blueprints/Interactables/TextHolders/BP_TextHolder_Parent` _array_element))
    (`self.UniversalStateSetter` _asbp_text_holder_parent)
    (`self.DestroyItem`)
    (return (`self.ItemName`) (`self.ItemDescription`))))

(fn `UniversalStateSetter`
  (params (HolderChanged :type "/Game/Blueprints/Interactables/TextHolders/BP_TextHolder_Parent Object Reference") (NewState :type Integer))
  (`GameplayStatics.GetAllActorsOfClass` (`GameplayStatics.GetObjectClass` HolderChanged))
  (`/Game/Blueprints/Interactables/TextHolders/BP_TextHolder_Parent.SetUniqueState` HolderChanged NewState))

(fn `UserConstructionScript`
  (locals (NewLocalVar :type "StaticMesh Object Reference"))
  (`StaticMeshComponent.SetStaticMesh` (`self.Sphere`) (`self.ItemModel`)))