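; BP_Item_Test is an interactable item that changes the state of a BP_Test character when obtained.
; ObtainItem finds all BP_Test actors, passes the first to UniversalStateSetter with a fixed new state, calls DestroyItem, then returns the item's name and description from inside the loop.
; A separate custom event destroys the actor after a short delay, and the construction script only runs the parent's.
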(event `CustomEvent`
  (`KismetSystemLibrary.Delay` 0.1)
  (`self.K2_DestroyActor`))

(fn `ObtainItem`
  (returns (ItemName :type String) (ItemDesciption :type String))
  ;[1 1 1] Change the state of one character
  (bind _outactors (`GameplayStatics.GetAllActorsOfClass` "/Game/Blueprints/Interactables/TextHolders/BP_Test.BP_Test_C"))
  (for _array_element _outactors
    (bind _asbp_test (cast `/Game/Blueprints/Interactables/TextHolders/BP_Test` _array_element))
    (`self.UniversalStateSetter` _asbp_test 4)
    (`self.DestroyItem`)
    (return (`self.ItemName`) (`self.ItemDescription`))))

(fn `UserConstructionScript`
  (`parent.UserConstructionScript`))