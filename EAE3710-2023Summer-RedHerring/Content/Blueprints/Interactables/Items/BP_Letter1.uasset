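; BP_Letter1 is an interactable letter item that changes a text holder's state and then removes itself.
; NewFunction fetches all BP_TextHolder_Parent actors, but returns within the first loop pass after resetting that holder to state 0 via UniversalStateSetter.
; It also calls DestroyItem and returns the item's name and description.
; A separate custom event destroys the actor after a short delay.
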(event `CustomEvent`
  (`KismetSystemLibrary.Delay` 0.1)
  (`self.K2_DestroyActor`))

(fn `NewFunction`
  (returns (ItemName :type String) (ItemDesciption :type String))
  ;[1 1 1] Change the state of one character
  (bind _outactors (`GameplayStatics.GetAllActorsOfClass` "/Game/Blueprints/Interactables/TextHolders/BP_TextHolder_Parent.BP_TextHolder_Parent_C"))
  (for _array_element _outactors
    (bind _asbp_text_holder_parent (cast `/Game/Blueprints/Interactables/TextHolders/BP_TextHolder_Parent` _array_element))
    (`self.UniversalStateSetter` _asbp_text_holder_parent)
    (`self.DestroyItem`)
    (return (`self.ItemName`) (`self.ItemDescription`))))

(fn `UserConstructionScript`
  (`parent.UserConstructionScript`))