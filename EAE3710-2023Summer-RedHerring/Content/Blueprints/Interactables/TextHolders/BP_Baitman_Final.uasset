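; Baitman NPC that runs branching dialogue and turns to face the player every tick.
; DisplayText steps through state line ranges from map keys and values, showing text and speaker in WB_DisplayText while blocking movement.
; State 1 opens a mouse-driven options menu; other states loop, advance or return to it.
; Branch-completion flags unlock state 7, and SetUniqueState jumps to any state's first line.
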(event `self.DisplayText`
  (bind _returnvalue (`GameplayStatics.GetPlayerController` 0))
  (bind _returnvalue_2 (`GameplayStatics.GetPlayerController` 0))
  (bind _currentstate_bait (`self.CurrentState_Bait`))
  (bind _dialog_bait (`self.Dialog_Bait`))
  (bind _currentline_bait (`self.CurrentLine_Bait`))
  (bind _dialogstatese_bait (`self.DialogStateSE_Bait`))
  (bind _returnvalue_3 (`KismetStringLibrary.Conv_IntToString` (`self.CurrentState_Bait`)))
  ;[1 1 1] Dialogue System - Controls what dialogue box is current, the current state of dialogue, whether it loops, etc
  (switch `string` (`KismetStringLibrary.Conv_IntToString` _currentstate_bait)
    (:`Default`
      (bind _values (`BlueprintMapLibrary.Map_Values` _dialogstatese_bait))
      (bind _keys (`BlueprintMapLibrary.Map_Keys` _dialogstatese_bait))
      (bind _output (`|GetArrayItem` _values _currentstate_bait))
      (if (< _currentline_bait _output)
        (`/Engine/EditorBlueprintResources/StandardMacros.IncrementInt` _currentline_bait
          (:`  `
            (bind _keys_2 (`BlueprintMapLibrary.Map_Keys` _dialog_bait))
            (bind _values_2 (`BlueprintMapLibrary.Map_Values` _dialog_bait))
            ;[1 1 1] Text Display on Screen
            (bind _ui (`self.UI`)
              (:`then`
                _)
              (:`else`
                (bind _returnvalue_4 (`|CreateWidget` "/Game/UI/WB_DisplayText.WB_DisplayText_C" (`GameplayStatics.GetPlayerController` 0)))
                (bind _output_get (set `self.UI` _returnvalue_4))
                (`UserWidget.AddToViewport` _output_get 0)))
            (`RichTextBlock.SetText` (`/Game/UI/WB_DisplayText.DialogueText` _ui) (`KismetTextLibrary.Conv_StringToText` (`|GetArrayItem` _keys_2 _currentline_bait)))
            (`TextBlock.SetText` (`/Game/UI/WB_DisplayText.NameText` _ui) (`KismetTextLibrary.Conv_StringToText` (`|GetArrayItem` _values_2 _currentline_bait)))
            (`WidgetBlueprintLibrary.SetInputMode_GameAndUIEx` _returnvalue null)
            (`Controller.SetIgnoreMoveInput` _returnvalue true)))
        (elif (== _currentline_bait _output)
          (if (`|GetArrayItem` (`self.LoopingState_Bait`) _currentstate_bait)
            (set `self.CurrentLine_Bait` (`|GetArrayItem` _keys _currentstate_bait))
            (else
              (switch `string` _returnvalue_3
                (:`Default`
                  (`/Engine/EditorBlueprintResources/StandardMacros.IncrementInt` _currentstate_bait
                    (:`  `
                      (`/Engine/EditorBlueprintResources/StandardMacros.IncrementInt` _currentline_bait
                        (:`  `
                          _)))))
                (:`2`
                  (set `self.State1Bool` true)
                  (switch `string` _returnvalue_3
                    (:`4`
                      (set `self.State3Bool` true))
                    (:`5`
                      (set `self.State4Bool` true)))
                  (set `self.CurrentState_Bait` 1)
                  (set `self.CurrentLine_Bait` (`|GetArrayItem` _keys (stale _output_get_2)) :!label _label))
                (:`6`
                  (set `self.State2Bool` true)
                  (bind _output_get_2 (set `self.CurrentState_Bait` 1))
                  (goto _label)))))
          (`self.HideUI`)
          (if (and (`self.State1Bool`) (`self.State2Bool`))
            (bind _output_get_3 (set `self.CurrentState_Bait` 7))
            (bind _keys_3 (`BlueprintMapLibrary.Map_Keys` (`self.DialogStateSE_Bait`)))
            (set `self.CurrentLine_Bait` (`|GetArrayItem` _keys_3 _output_get_3))
            (set `self.State1Bool` false)
            (set `self.State2Bool` false)
            (elif (or (`self.State3Bool`) (`self.State4Bool`))
              (set `self.State3Bool` false)
              (set `self.State4Bool` false))))))
    (:`1`
      ;[1 1 1] First Dialogue Options
      (bind _returnvalue_5 (`|CreateWidget` "/Game/UI/WB_DisplayText.WB_DisplayText_C" _returnvalue_2))
      (bind _output_get_4 (set `self.UI` _returnvalue_5))
      (`UserWidget.AddToViewport` _output_get_4 0)
      (`WidgetBlueprintLibrary.SetInputMode_UIOnlyEx` _returnvalue_2 null)
      (`Controller.SetIgnoreMoveInput` _returnvalue_2 true)
      (set `PlayerController.bShowMouseCursor` true _returnvalue_2)
      (`WidgetSwitcher.SetActiveWidgetIndex` (`/Game/UI/WB_DisplayText.WidgetSwitcherText` _returnvalue_5) 6))))

(event `self.SetUniqueState`
  (params (NewState :type Integer))
  ;[1 1 1] Sets the state and line of this particular object
  (set `self.CurrentState_Bait` NewState)
  (bind _keys (`BlueprintMapLibrary.Map_Keys` (`self.DialogStateSE_Bait`)))
  (set `self.CurrentLine_Bait` (`|GetArrayItem` _keys NewState)))

(event `self.ReceiveTick`
  (params (DeltaSeconds :type "Float (single-precision)"))
  ;[1 1 1] Makes the character always face the player
  (`self.K2_SetActorRotation` self (`KismetMathLibrary.MakeRotator` (.roll (`KismetMathLibrary.FindLookAtRotation` (`self.K2_GetActorLocation` self) (`self.K2_GetActorLocation` (`GameplayStatics.GetPlayerCharacter` 0)))) 0.0 (.yaw (`KismetMathLibrary.FindLookAtRotation` (`self.K2_GetActorLocation` self) (`self.K2_GetActorLocation` (`GameplayStatics.GetPlayerCharacter` 0))))) false))

(fn `UserConstructionScript`
  (`parent.UserConstructionScript`))