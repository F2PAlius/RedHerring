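; Test dialogue interactable that always turns to face the player and shows its lines in WB_DisplayText.
; DisplayText steps through line ranges from DialogueStatesSETest, pulling text and speaker from DialogueTest, then loops or advances the state and hides the UI.
; State 4 opens a mouse-driven options screen; branches 5 and 6 return to it until both finish, unlocking state 7.
; SetUniqueState jumps to a given state and its first line.
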(event `self.DisplayText`
  (bind _returnvalue (`GameplayStatics.GetPlayerController` 0))
  (bind _returnvalue_2 (`GameplayStatics.GetPlayerController` 0))
  (bind _currentstatetest (`self.CurrentStateTest`))
  (bind _dialoguestatessetest (`self.DialogueStatesSETest`))
  (bind _currentlinetest (`self.CurrentLineTest`))
  (bind _dialoguetest (`self.DialogueTest`))
  (bind _currentlinetest_2 (`self.CurrentLineTest`))
  ;[1 1 1] Dialogue System - Controls what dialogue box is current, the current state of dialogue, whether it loops, etc
  (switch `string` (`KismetStringLibrary.Conv_IntToString` (`self.CurrentStateTest`))
    (:`Default`
      (bind _values (`BlueprintMapLibrary.Map_Values` _dialoguestatessetest))
      (bind _keys (`BlueprintMapLibrary.Map_Keys` _dialoguestatessetest))
      (bind _output (`|GetArrayItem` _values _currentstatetest))
      (if (< _currentlinetest_2 _output)
        (`/Engine/EditorBlueprintResources/StandardMacros.IncrementInt` _currentlinetest
          (:`  `
            (bind _keys_2 (`BlueprintMapLibrary.Map_Keys` _dialoguetest))
            (bind _values_2 (`BlueprintMapLibrary.Map_Values` _dialoguetest))
            ;[1 1 1] Text Display on Screen
            (bind _ui (`self.UI`)
              (:`then`
                _)
              (:`else`
                (bind _returnvalue_3 (`|CreateWidget` "/Game/UI/WB_DisplayText.WB_DisplayText_C" (`GameplayStatics.GetPlayerController` 0)))
                (bind _output_get (set `self.UI` _returnvalue_3))
                (`UserWidget.AddToViewport` _output_get 0)))
            (`RichTextBlock.SetText` (`/Game/UI/WB_DisplayText.DialogueText` _ui) (`KismetTextLibrary.Conv_StringToText` (`|GetArrayItem` _keys_2 _currentlinetest)))
            (`TextBlock.SetText` (`/Game/UI/WB_DisplayText.NameText` _ui) (`KismetTextLibrary.Conv_StringToText` (`|GetArrayItem` _values_2 _currentlinetest)))
            (`WidgetBlueprintLibrary.SetInputMode_GameAndUIEx` _returnvalue null)
            (`Controller.SetIgnoreMoveInput` _returnvalue true)))
        (elif (== _currentlinetest_2 _output)
          (if (`|GetArrayItem` (`self.LoopingStatesTest`) _currentstatetest)
            (set `self.CurrentLineTest` (`|GetArrayItem` _keys _currentstatetest))
            (else
              (switch `string` (`KismetStringLibrary.Conv_IntToString` (`self.CurrentStateTest`))
                (:`Default`
                  (`/Engine/EditorBlueprintResources/StandardMacros.IncrementInt` _currentstatetest
                    (:`  `
                      (`/Engine/EditorBlueprintResources/StandardMacros.IncrementInt` _currentlinetest
                        (:`  `
                          _)))))
                (:`5`
                  (set `self.5Finished` true)
                  (bind _output_get_2 (set `self.CurrentStateTest` 4 :!label _label))
                  (set `self.CurrentLineTest` (`|GetArrayItem` _keys _output_get_2)))
                (:`6`
                  (set `self.6Finished` true)
                  (goto _label)))))
          (`self.HideUI`)
          (if (and (`self.5Finished`) (`self.6Finished`))
            (bind _output_get_3 (set `self.CurrentStateTest` 7))
            (bind _keys_3 (`BlueprintMapLibrary.Map_Keys` (`self.DialogueStatesSETest`)))
            (set `self.CurrentLineTest` (`|GetArrayItem` _keys_3 _output_get_3))
            (set `self.5Finished` false)
            (set `self.6Finished` false)))))
    (:`4`
      ;[1 1 1] First Dialogue Options
      (bind _returnvalue_4 (`|CreateWidget` "/Game/UI/WB_DisplayText.WB_DisplayText_C" _returnvalue_2))
      (bind _output_get_4 (set `self.UI` _returnvalue_4))
      (`UserWidget.AddToViewport` _output_get_4 0)
      (`WidgetBlueprintLibrary.SetInputMode_UIOnlyEx` _returnvalue_2 null)
      (`Controller.SetIgnoreMoveInput` _returnvalue_2 true)
      (set `PlayerController.bShowMouseCursor` true _returnvalue_2)
      (`WidgetSwitcher.SetActiveWidgetIndex` (`/Game/UI/WB_DisplayText.WidgetSwitcherText` _returnvalue_4) 2))))

(event `self.SetUniqueState`
  (params (NewState :type Integer))
  ;[1 1 1] Sets the state and line of this particular object
  (set `self.CurrentStateTest` NewState)
  (bind _keys (`BlueprintMapLibrary.Map_Keys` (`self.DialogueStatesSETest`)))
  (set `self.CurrentLineTest` (`|GetArrayItem` _keys NewState)))

(event `self.HideUI`
  (bind _returnvalue (`GameplayStatics.GetPlayerController` 0))
  (bind _ui (`self.UI`))
  ;[1 1 1] Simple UI Hiding
  (`self.UI`
    (:`then`
      (`Widget.RemoveFromParent` _ui)
      (`WidgetSwitcher.SetActiveWidgetIndex` (`/Game/UI/WB_DisplayText.WidgetSwitcherText` _ui) 0)
      (set `self.UI` null)
      (`WidgetBlueprintLibrary.SetInputMode_GameOnly` _returnvalue)
      (set `PlayerController.bShowMouseCursor` false _returnvalue)
      (`Controller.ResetIgnoreMoveInput` _returnvalue))
    (:`else`)))

(event `self.ReceiveTick`
  (params (DeltaSeconds :type "Float (single-precision)"))
  ;[1 1 1] Makes the character always face the player
  (`self.K2_SetActorRotation` self (`KismetMathLibrary.MakeRotator` (.roll (`KismetMathLibrary.FindLookAtRotation` (`self.K2_GetActorLocation` self) (`self.K2_GetActorLocation` (`GameplayStatics.GetPlayerCharacter` 0)))) 0.0 (.yaw (`KismetMathLibrary.FindLookAtRotation` (`self.K2_GetActorLocation` self) (`self.K2_GetActorLocation` (`GameplayStatics.GetPlayerCharacter` 0))))) false))

(fn `UserConstructionScript`
  (`parent.UserConstructionScript`))