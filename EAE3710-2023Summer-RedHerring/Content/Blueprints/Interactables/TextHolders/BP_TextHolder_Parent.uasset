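; Parent Blueprint for dialogue-holding interactables that turn to face the player every tick with pitch zeroed.
; Each DisplayText call advances through the current state's line range, showing text and speaker from the Dialogue map in WB_DisplayText while blocking movement.
; At a range's end it loops or moves to the next state, then hides the UI and restores input.
; SetUniqueState jumps directly to a given state's first line.
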(event `self.DisplayText`
  (bind _returnvalue (`GameplayStatics.GetPlayerController` 0))
  (bind _currentline (`self.CurrentLine`))
  (bind _currentstate (`self.CurrentState`))
  (bind _dialogue (`self.Dialogue`))
  (bind _dialoguestatesstartend (`self.DialogueStatesStartEnd`))
  (bind _currentline_2 (`self.CurrentLine`))
  ;[1 1 1] Dialogue System - Controls what dialogue box is current, the current state of dialogue, whether it loops, etc
  (bind _values (`BlueprintMapLibrary.Map_Values` _dialoguestatesstartend))
  (bind _keys (`BlueprintMapLibrary.Map_Keys` _dialoguestatesstartend))
  (bind _output (`|GetArrayItem` _values _currentstate))
  (if (< _currentline_2 _output)
    (`/Engine/EditorBlueprintResources/StandardMacros.IncrementInt` _currentline
      (:`  `
        (bind _keys_2 (`BlueprintMapLibrary.Map_Keys` _dialogue))
        (bind _values_2 (`BlueprintMapLibrary.Map_Values` _dialogue))
        ;[1 1 1] Text Display on Screen
        (bind _ui (`self.UI`)
          (:`then`
            _)
          (:`else`
            (bind _returnvalue_2 (`|CreateWidget` "/Game/UI/WB_DisplayText.WB_DisplayText_C" (`GameplayStatics.GetPlayerController` 0)))
            (bind _output_get (set `self.UI` _returnvalue_2))
            (`UserWidget.AddToViewport` _output_get 0)))
        (`RichTextBlock.SetText` (`/Game/UI/WB_DisplayText.DialogueText` _ui) (`KismetTextLibrary.Conv_StringToText` (`|GetArrayItem` _keys_2 _currentline)))
        (`TextBlock.SetText` (`/Game/UI/WB_DisplayText.NameText` _ui) (`KismetTextLibrary.Conv_StringToText` (`|GetArrayItem` _values_2 _currentline)))
        (`WidgetBlueprintLibrary.SetInputMode_GameAndUIEx` _returnvalue null)
        (`Controller.SetIgnoreMoveInput` _returnvalue true)))
    (elif (== _currentline_2 _output)
      (if (`|GetArrayItem` (`self.LoopingStates`) _currentstate)
        (set `self.CurrentLine` (`|GetArrayItem` _keys _currentstate))
        (else
          (switch `string` ""
            (:`Default`
              (`/Engine/EditorBlueprintResources/StandardMacros.IncrementInt` _currentstate
                (:`  `
                  (`/Engine/EditorBlueprintResources/StandardMacros.IncrementInt` _currentline
                    (:`  `
                      _))))))))
      (`self.HideUI`))))

(event `self.SetUniqueState`
  (params (NewState :type Integer))
  ;[1 1 1] Sets the state and line of this particular object
  (set `self.CurrentState` NewState)
  (bind _keys (`BlueprintMapLibrary.Map_Keys` (`self.DialogueStatesStartEnd`)))
  (set `self.CurrentLine` (`|GetArrayItem` _keys NewState)))

(event `self.HideUI`
  (bind _returnvalue (`GameplayStatics.GetPlayerController` 0))
  (bind _ui (`self.UI`))
  ;[1 1 1] Simple UI Hiding
  (`self.UI`
    (:`then`
      (`Widget.RemoveFromParent` _ui)
      (`WidgetSwitcher.SetActiveWidgetIndex` (`/Game/UI/WB_DisplayText.WidgetSwitcherText` _ui) 0)
      (set `self.UI` null)
      (`WidgetBlueprintLibrary.SetInputMode_GameOnly` _returnvalue)
      (set `PlayerController.bShowMouseCursor` false _returnvalue)
      (`Controller.ResetIgnoreMoveInput` _returnvalue))
    (:`else`)))

(event `self.ReceiveTick`
  (params (DeltaSeconds :type "Float (single-precision)"))
  ;[1 1 1] Makes the character always face the player
  (`self.K2_SetActorRotation` self (`KismetMathLibrary.MakeRotator` (.roll (`KismetMathLibrary.FindLookAtRotation` (`self.K2_GetActorLocation` self) (`self.K2_GetActorLocation` (`GameplayStatics.GetPlayerCharacter` 0)))) 0.0 (.yaw (`KismetMathLibrary.FindLookAtRotation` (`self.K2_GetActorLocation` self) (`self.K2_GetActorLocation` (`GameplayStatics.GetPlayerCharacter` 0))))) false))

(fn `UserConstructionScript`)