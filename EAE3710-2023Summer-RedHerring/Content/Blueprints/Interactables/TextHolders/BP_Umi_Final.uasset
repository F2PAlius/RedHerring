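; Interactable NPC Umi, who runs a branching dialogue through WB_DisplayText and turns to face the player every tick.
; DisplayText steps through line and speaker maps within per-state ranges, blocking movement and looping or advancing states at each range's end.
; State 1 opens a choice panel; finished non-looping branches 2 and 3 return there, unlocking state 4 once both complete.
; SetUniqueState jumps to a given state's first line.
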(event `self.DisplayText`
  (bind _returnvalue (`GameplayStatics.GetPlayerController` 0))
  (bind _returnvalue_2 (`GameplayStatics.GetPlayerController` 0))
  (bind _currentstate_umi (`self.CurrentState_Umi`))
  (bind _currentline_umi (`self.CurrentLine_Umi`))
  (bind _dialogstatese_umi (`self.DialogStateSE_Umi`))
  (bind _dialog_umi (`self.Dialog_Umi`))
  (bind _currentline_umi_2 (`self.CurrentLine_Umi`))
  ;[1 1 1] Dialogue System - Controls what dialogue box is current, the current state of dialogue, whether it loops, etc
  (switch `string` (`KismetStringLibrary.Conv_IntToString` _currentstate_umi)
    (:`Default`
      (bind _values (`BlueprintMapLibrary.Map_Values` _dialogstatese_umi))
      (bind _keys (`BlueprintMapLibrary.Map_Keys` _dialogstatese_umi))
      (bind _output (`|GetArrayItem` _values _currentstate_umi))
      (if (< _currentline_umi _output)
        (`/Engine/EditorBlueprintResources/StandardMacros.IncrementInt` _currentline_umi_2
          (:`  `
            (bind _keys_2 (`BlueprintMapLibrary.Map_Keys` _dialog_umi))
            (bind _values_2 (`BlueprintMapLibrary.Map_Values` _dialog_umi))
            ;[1 1 1] Text Display on Screen
            (bind _ui (`self.UI`)
              (:`then`
                _)
              (:`else`
                (bind _returnvalue_3 (`|CreateWidget` "/Game/UI/WB_DisplayText.WB_DisplayText_C" (`GameplayStatics.GetPlayerController` 0)))
                (bind _output_get (set `self.UI` _returnvalue_3))
                (`UserWidget.AddToViewport` _output_get 0)))
            (`RichTextBlock.SetText` (`/Game/UI/WB_DisplayText.DialogueText` _ui) (`KismetTextLibrary.Conv_StringToText` (`|GetArrayItem` _keys_2 _currentline_umi_2)))
            (`TextBlock.SetText` (`/Game/UI/WB_DisplayText.NameText` _ui) (`KismetTextLibrary.Conv_StringToText` (`|GetArrayItem` _values_2 _currentline_umi_2)))
            (`WidgetBlueprintLibrary.SetInputMode_GameAndUIEx` _returnvalue null)
            (`Controller.SetIgnoreMoveInput` _returnvalue true)))
        (elif (== _currentline_umi _output)
          (if (`|GetArrayItem` (`self.LoopingStates_Umi`) _currentstate_umi)
            (set `self.CurrentLine_Umi` (`|GetArrayItem` _keys _currentstate_umi))
            (else
              (switch `string` (`KismetStringLibrary.Conv_IntToString` (`self.CurrentState_Umi`))
                (:`Default`
                  (`/Engine/EditorBlueprintResources/StandardMacros.IncrementInt` _currentstate_umi
                    (:`  `
                      (`/Engine/EditorBlueprintResources/StandardMacros.IncrementInt` _currentline_umi_2
                        (:`  `
                          _)))))
                (:`2`
                  (set `self.State1Bool` true)
                  (bind _output_get_2 (set `self.CurrentState_Umi` 1 :!label _label))
                  (set `self.CurrentLine_Umi` (`|GetArrayItem` _keys _output_get_2)))
                (:`3`
                  (set `self.State2Bool` true)
                  (goto _label)))))
          (`self.HideUI`)
          (if (and (`self.State1Bool`) (`self.State2Bool`))
            (bind _output_get_3 (set `self.CurrentState_Umi` 4))
            (bind _keys_3 (`BlueprintMapLibrary.Map_Keys` (`self.DialogStateSE_Umi`)))
            (set `self.CurrentLine_Umi` (`|GetArrayItem` _keys_3 _output_get_3))
            (set `self.State1Bool` false)
            (set `self.State2Bool` false)))))
    (:`1`
      ;[1 1 1] First Dialogue Options
      (bind _returnvalue_4 (`|CreateWidget` "/Game/UI/WB_DisplayText.WB_DisplayText_C" _returnvalue_2))
      (bind _output_get_4 (set `self.UI` _returnvalue_4))
      (`UserWidget.AddToViewport` _output_get_4 0)
      (`WidgetBlueprintLibrary.SetInputMode_UIOnlyEx` _returnvalue_2 null)
      (`Controller.SetIgnoreMoveInput` _returnvalue_2 true)
      (set `PlayerController.bShowMouseCursor` true _returnvalue_2)
      (`WidgetSwitcher.SetActiveWidgetIndex` (`/Game/UI/WB_DisplayText.WidgetSwitcherText` _returnvalue_4) 3))))

(event `self.SetUniqueState`
  (params (NewState :type Integer))
  ;[1 1 1] Sets the state and line of this particular object
  (set `self.CurrentState_Umi` NewState)
  (bind _keys (`BlueprintMapLibrary.Map_Keys` (`self.DialogStateSE_Umi`)))
  (set `self.CurrentLine_Umi` (`|GetArrayItem` _keys NewState)))

(event `self.ReceiveTick`
  (params (DeltaSeconds :type "Float (single-precision)"))
  ;[1 1 1] Makes the character always face the player
  (`self.K2_SetActorRotation` self (`KismetMathLibrary.MakeRotator` (.roll (`KismetMathLibrary.FindLookAtRotation` (`self.K2_GetActorLocation` self) (`self.K2_GetActorLocation` (`GameplayStatics.GetPlayerCharacter` 0)))) 0.0 (.yaw (`KismetMathLibrary.FindLookAtRotation` (`self.K2_GetActorLocation` self) (`self.K2_GetActorLocation` (`GameplayStatics.GetPlayerCharacter` 0))))) false))

(fn `UserConstructionScript`
  (`parent.UserConstructionScript`))